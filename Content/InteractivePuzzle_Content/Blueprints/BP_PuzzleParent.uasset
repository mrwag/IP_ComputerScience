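; Base actor for lever-driven code puzzles, where child classes override RunCode and ResetCode to build block solutions.
; Lever interaction alternates between running the code and resetting, while the construction script grid-snaps the actor, labels it from its class name and wires the lever.
; PlaceBlockOfType spawns hidden blocks into an array, which looping timers reveal one by one, then on reset hide in reverse order and destroy.
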(event Custom|FinishAndShowSolution
  (Components|Timeline|PlayfromStart (Variables|Default|GetBannerMovement))
  (Variables|Default|SetCurrentIndex 0)
  (if (> (Utilities|Array|Length (Variables|Default|GetBlockBuildArray)) 0)
    (Utilities|Time|SetTimerbyEvent (delegate Custom|PlaceBlock) 0.1 true)
    (Rendering|SetActorHiddenInGame (Utilities|Array|Get(acopy) (Variables|Default|GetBlockBuildArray) (Variables|Default|GetCurrentIndex)) false)
    (bind _result (Math|Integer|IncrementInt (Variables|Default|GetCurrentIndex))
      (:%20%20
        (if (> _result (Utilities|Array|LastIndex (Variables|Default|GetBlockBuildArray)))
          (Utilities|Time|ClearTimerbyFunctionName 0 "PlaceBlock"))))))

(event Custom|PlaceBlock
  (Rendering|SetActorHiddenInGame (Utilities|Array|Get(acopy) (Variables|Default|GetBlockBuildArray) (Variables|Default|GetCurrentIndex)) false)
  (bind _result (Math|Integer|IncrementInt (Variables|Default|GetCurrentIndex))
    (:%20%20
      (if (> _result (Utilities|Array|LastIndex (Variables|Default|GetBlockBuildArray)))
        (Utilities|Time|ClearTimerbyFunctionName 0 "PlaceBlock")))))

(event Custom|ResetPuzzle
  (bind _blockbuildarray (Variables|Default|GetBlockBuildArray))
  (Components|Timeline|ReversefromEnd (Variables|Default|GetBannerMovement))
  (CallFunction|ResetCode)
  (if (> (Utilities|Array|Length (Variables|Default|GetBlockBuildArray)) 0)
    (Utilities|Time|SetTimerbyEvent (delegate Custom|RemoveCustomBlocks) 0.05 true)
    (Utilities|IsValid (Utilities|Array|Get(acopy) (Variables|Default|GetBlockBuildArray) (Variables|Default|GetCurrentIndex))
      (:Is%20Valid
        (Rendering|SetActorHiddenInGame (Utilities|Array|Get(acopy) (Variables|Default|GetBlockBuildArray) (Variables|Default|GetCurrentIndex)) true))
      (:Is%20Not%20Valid
        _))
    (bind _result (Math|Integer|DecrementInt (Variables|Default|GetCurrentIndex))
      (:%20%20
        (if (< _result 0)
          (Utilities|Time|ClearTimerbyFunctionName 0 "RemoveCustomBlocks")
          (Actor|DestroyActor _blockbuildarray)
          (Utilities|Array|Clear _blockbuildarray)
          (Variables|Default|SetCurrentIndex 0)
          (CallFunction|ChangeMessage "Interact with Lever to run code!"))))))

(event Custom|RemoveCustomBlocks
  (bind _blockbuildarray (Variables|Default|GetBlockBuildArray))
  (Utilities|IsValid (Utilities|Array|Get(acopy) (Variables|Default|GetBlockBuildArray) (Variables|Default|GetCurrentIndex))
    (:Is%20Valid
      (Rendering|SetActorHiddenInGame (Utilities|Array|Get(acopy) (Variables|Default|GetBlockBuildArray) (Variables|Default|GetCurrentIndex)) true))
    (:Is%20Not%20Valid
      _))
  (bind _result (Math|Integer|DecrementInt (Variables|Default|GetCurrentIndex))
    (:%20%20
      (if (< _result 0)
        (Utilities|Time|ClearTimerbyFunctionName 0 "RemoveCustomBlocks")
        (Actor|DestroyActor _blockbuildarray)
        (Utilities|Array|Clear _blockbuildarray)
        (Variables|Default|SetCurrentIndex 0)
        (CallFunction|ChangeMessage "Interact with Lever to run code!")))))

(event EventBeginPlay)

(event EventInteractwith
  (bind _blockbuildarray (Variables|Default|GetBlockBuildArray))
  (Utilities|FlowControl|FlipFlop
    (:A
      (Utilities|Time|ClearTimerbyFunctionName 0 "PlaceBlock")
      (Utilities|Time|ClearTimerbyFunctionName 0 "RemoveCustomBlocks")
      (Actor|DestroyActor _blockbuildarray)
      (Variables|Default|SetCurrentIndex 0)
      (Utilities|Array|Clear _blockbuildarray)
      (CallFunction|InitiateSolution))
    (:B
      (Utilities|Time|ClearTimerbyFunctionName 0 "PlaceBlock")
      (Utilities|Time|ClearTimerbyFunctionName 0 "RemoveCustomBlocks")
      (CallFunction|ResetPuzzle))))

(fn ConstructionScript
  (bind _returnvalue (Transformation|GetActorLocation))
  (bind _self self)
  (bind _returnvalue_2 (Utilities|GetClass _self))
  (bind _returnvalue_3 (Utilities|GetClassDisplayName _returnvalue_2))
  (|CallParentFunction)
  (Transformation|SetActorLocation (Math|Vector|MakeVector (Math|Float|SnapToGrid(Float) (.x _returnvalue) 1e+02) (Math|Float|SnapToGrid(Float) (.y _returnvalue) 1e+02) (.z _returnvalue)) false false)
  (Rendering|Components|TextRender|SetText (Variables|Default|GetPuzzleLabel) (Utilities|Text|ToText(String) (Utilities|String|GetSubstring _returnvalue_3 0 (- (Utilities|String|Len _returnvalue_3) 2))))
  (bind _aslever_bp (Utilities|Casting|CastToLever_BP (Variables|/Script/Engine.ChildActorComponent|GetChildActor (Variables|Default|GetBP_Lever))))
  (Variables|/Game/ULK_Games/Blueprints/Interactables/Lever_BP.Lever_BP_C|SetInteractable _aslever_bp self)
  (Variables|/Game/ULK_Games/Blueprints/Interactables/Lever_BP.Lever_BP_C|SetLeverSpeed _aslever_bp 2.0)
  (Transformation|SetWorldScale3D (Variables|Default|GetFloorMesh) (Math|Vector|MakeVector (* (Variables|Default|GetFloorX) 0.25) (* (Variables|Default|GetFloorY) 0.25) 1.0)))

(fn ChangeMessage
  (params (NewMessage :type String))
  (Rendering|Components|TextRender|SetText (Variables|Default|GetMessage) (Utilities|Text|ToText(String) NewMessage)))

(fn RunCode)

(fn PlaceBlockOfType
  (params (RelativeLocation :type Vector) (BlockType :type E_BlockTypes%20Enum :default "NewEnumerator0"))
  (bind _returnvalue (Game|SpawnActorfromClass (Utilities|Select :Index BlockType :NewEnumerator0 "/Game/InteractivePuzzle_Content/Blueprints/BlockBP/BP_RedBlock.BP_RedBlock_C" :NewEnumerator1 "/Game/InteractivePuzzle_Content/Blueprints/BlockBP/BP_GreenBlock.BP_GreenBlock_C" :NewEnumerator2 "/Game/InteractivePuzzle_Content/Blueprints/BlockBP/BP_BlueBlock.BP_BlueBlock_C" :NewEnumerator3 "/Game/InteractivePuzzle_Content/Blueprints/BlockBP/BP_GrassBlock.BP_GrassBlock_C" :NewEnumerator4 "/Game/InteractivePuzzle_Content/Blueprints/BlockBP/BP_StoneBlock.BP_StoneBlock_C" :NewEnumerator5 "/Game/InteractivePuzzle_Content/Blueprints/BlockBP/BP_Purple.BP_Purple_C" :NewEnumerator6 "/Game/InteractivePuzzle_Content/Blueprints/BlockBP/BP_Gold.BP_Gold_C" :NewEnumerator7 "/Game/InteractivePuzzle_Content/Blueprints/BlockBP/BP_Teal.BP_Teal_C" :NewEnumerator8 "/Game/InteractivePuzzle_Content/Blueprints/BlockBP/BP_Green.BP_Green_C" :NewEnumerator9 "/Game/InteractivePuzzle_Content/Blueprints/BlockBP/BP_WoodCrate.BP_WoodCrate_C") (Math|Transform|MakeTransform (+ RelativeLocation (Transformation|GetActorLocation)) "0, 0, 0" "1,1,1") "Undefined" 0 0))
  (Rendering|SetActorHiddenInGame _returnvalue true)
  (bind _asbp_block_parent (Utilities|Casting|CastToBP_BlockParent _returnvalue))
  (Utilities|Array|Add (Variables|Default|GetBlockBuildArray) _asbp_block_parent))

(fn InitiateSolution
  ;[1 1 1] RunCode is implemented in the child class
  (CallFunction|RunCode)
  ;[1 1 1] Show the result
  (CallFunction|FinishandShowSolution))

(fn ResetCode)