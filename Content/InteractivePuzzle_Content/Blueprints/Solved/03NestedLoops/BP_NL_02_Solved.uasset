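; Solved version of the second nested-loops puzzle in the interactive puzzle content, building a triangular staircase of blocks.
; RunCode triggers the PuzzleSolution event, which runs an outer loop along Y and an inner loop up Z bounded by the current outer index.
; Each iteration calls PlaceBlockOfType with a single block type on a 100-unit grid, so columns grow taller along Y.
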(event Custom|PuzzleSolution
  (for _index (range 0 5)
    (Variables|Default|Sety _index)
    (for _index_2 (range 0 (Variables|Default|Gety))
      (Variables|Default|Setz _index_2)
      (CallFunction|PlaceBlockOfType (Math|Vector|MakeVector 0.0 (* (Variables|Default|Gety) 1e+02) (* (Variables|Default|Getz) 1e+02)) "NewEnumerator6"))))

(event EventBeginPlay)

(event Collision|EventActorBeginOverlap
  (params (OtherActor :type Actor%20Object%20Reference)))

(event EventTick
  (params (DeltaSeconds :type Float%20%28single-precision%29)))

(fn ConstructionScript
  (|CallParentFunction))

(fn RunCode
  (CallFunction|PuzzleSolution))