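; Solved version of a nested-loops puzzle that builds a wall-like block pattern with alternating tall and short columns.
; RunCode calls PuzzleSolution, whose outer loop steps along Y and uses a modulo check to set each column's height, tall on even indices and a single block on odd ones.
; The inner loop stacks blocks of one type up Z on a 100-unit grid through PlaceBlockOfType.
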(event Custom|PuzzleSolution
  (for _index (range 0 6)
    (Variables|Default|Sety _index)
    (if (== (Math|Integer|%(Integer) (Variables|Default|Gety) 2) 0)
      (Variables|Default|SetHeight 5)
      (else
        (Variables|Default|SetHeight 0)))
    (for _index_2 (range 0 (Variables|Default|GetHeight))
      (Variables|Default|Setz _index_2)
      (CallFunction|PlaceBlockOfType (Math|Vector|MakeVector 0.0 (* (Variables|Default|Gety) 1e+02) (* (Variables|Default|Getz) 1e+02)) "NewEnumerator8"))))

(fn ConstructionScript
  (|CallParentFunction))

(fn RunCode
  (CallFunction|PuzzleSolution))