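; Solved Blueprint for the first nested-loop puzzle, which builds a square wall of blocks of a single type.
; RunCode triggers PuzzleSolution, where an outer loop steps along Y and an inner loop along Z.
; Each iteration calls PlaceBlockOfType, scaling both indices by the block spacing to get relative locations on the vertical YZ plane.
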(event Custom|PuzzleSolution
  (for _index (range 0 5)
    (Variables|Default|Sety _index)
    (for _index_2 (range 0 5)
      (Variables|Default|Setz _index_2)
      (CallFunction|PlaceBlockOfType (Math|Vector|MakeVector 0.0 (* (Variables|Default|Gety) 1e+02) (* (Variables|Default|Getz) 1e+02)) "NewEnumerator7"))))

(fn ConstructionScript
  (|CallParentFunction))

(fn RunCode
  (CallFunction|PuzzleSolution))