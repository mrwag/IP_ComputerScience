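; BP_Var_02_Solved is the solved version of a variables exercise in the interactive puzzle content.
; RunCode fires the PuzzleSolution event, which sets Y to 1, places a block at a relative Y offset of Y times 100, increments Y, and places a block of another type one step further along.
; The construction script only calls its parent.
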(event Custom|PuzzleSolution
  (Variables|Default|SetY 1)
  (CallFunction|PlaceBlockOfType (Math|Vector|MakeVector 0.0 (* (Variables|Default|GetY) 1e+02) 0.0) "NewEnumerator4")
  (Math|Integer|IncrementInt (Variables|Default|GetY)
    (:%20%20
      (CallFunction|PlaceBlockOfType (Math|Vector|MakeVector 0.0 (* (Variables|Default|GetY) 1e+02) 0.0) "NewEnumerator3"))))

(fn ConstructionScript
  (|CallParentFunction))

(fn RunCode
  (CallFunction|PuzzleSolution))