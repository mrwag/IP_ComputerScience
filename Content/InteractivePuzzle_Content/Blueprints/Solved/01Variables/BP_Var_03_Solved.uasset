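; BP_Var_03_Solved is the solved version of a variables exercise in an interactive Blueprint puzzle set, showing a string variable driving on-screen text.
; RunCode fires the PuzzleSolution event, which sets MyName to "John" and passes it to the MyMessage text component.
; ResetCode calls the parent reset and restores the placeholder text, while the construction script only defers to the parent.
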(event Custom|PuzzleSolution
  (bind _output_get (Variables|Default|SetMyName "John"))
  (Rendering|Components|TextRender|SetText (Variables|Default|GetMyMessage) _output_get))

(fn ConstructionScript
  (|CallParentFunction))

(fn RunCode
  (CallFunction|PuzzleSolution))

(fn ResetCode
  (|CallParentFunction)
  (Rendering|Components|TextRender|SetText (Variables|Default|GetMyMessage) (Utilities|Text|MakeLiteralText "Change me!")))