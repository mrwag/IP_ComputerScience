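; Solved version of the third single-loop puzzle in an interactive Blueprint puzzle set, which builds a row of six blocks with alternating types.
; RunCode fires the PuzzleSolution event, which runs one for-loop over the block index.
; Each pass spaces a block evenly along relative Y through PlaceBlockOfType, using a modulo-two check on the index to pick between two block types.
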(event Custom|PuzzleSolution
  (Variables|Default|SetZ 0)
  (for _index (range 0 5)
    (bind _output_get (Variables|Default|Sety _index))
    (if (== (Math|Integer|%(Integer) _output_get 2) 0)
      (CallFunction|PlaceBlockOfType (Math|Vector|MakeVector 0.0 (* (Variables|Default|Gety) 1e+02) 0.0) "NewEnumerator6")
      (else
        (CallFunction|PlaceBlockOfType (Math|Vector|MakeVector 0.0 (* (Variables|Default|Gety) 1e+02) 0.0) "NewEnumerator5")))))

(fn ConstructionScript
  (|CallParentFunction))

(fn RunCode
  (CallFunction|PuzzleSolution))