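; Solved single-loop puzzle Blueprint, number 04, from an interactive puzzle set, placing blocks in a staggered pattern.
; RunCode fires PuzzleSolution, which loops over six indices to step along Y and uses index modulo 2 to alternate Z between two levels.
; Each iteration calls PlaceBlockOfType with one block type at that grid position, scaled to 100-unit spacing.
; The construction script only calls its parent.
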(event Custom|PuzzleSolution
  (Variables|Default|SetZ 0)
  (for _index (range 0 5)
    (bind _output_get (Variables|Default|Sety _index))
    (Variables|Default|SetZ (Math|Integer|%(Integer) _output_get 2))
    (CallFunction|PlaceBlockOfType (Math|Vector|MakeVector 0.0 (* (Variables|Default|Gety) 1e+02) (* (Variables|Default|GetZ) 1e+02)) "NewEnumerator6")))

(fn ConstructionScript
  (|CallParentFunction))

(fn RunCode
  (CallFunction|PuzzleSolution))