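; BP_NL_04_Start_SubGoal is the unsolved starter Blueprint for a nested-loop lesson puzzle about placing blocks in columns.
; RunCode calls an empty PuzzleSolution event.
; Disconnected scaffold pieces supply a seven-step Y loop, a column-height branch feeding a Z loop, and a block placement call.
; Loose math nodes offer coordinate scaling and an even-Y check, all unwired.
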(event Custom|PuzzleSolution)

(fn ConstructionScript
  (|CallParentFunction))

(fn RunCode
  (CallFunction|PuzzleSolution))