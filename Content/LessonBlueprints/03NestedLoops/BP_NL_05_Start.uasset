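; A nested-loop lesson Blueprint whose puzzle solution fills a box-shaped volume with blocks of a single type.
; RunCode calls the PuzzleSolution event, which runs three nested loops over Height, Width and Length to set Z, X and Y.
; The innermost loop calls PlaceBlockOfType at those indices scaled to a 100-unit grid, while the construction script only calls its parent.
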(event Custom|PuzzleSolution
  (for _index (range 0 (- (Variables|Default|GetHeight) 1))
    (Variables|Default|SetZ _index)
    (for _index_2 (range 0 (- (Variables|Default|GetWidth) 1))
      (Variables|Default|SetX _index_2)
      (for _index_3 (range 0 (- (Variables|Default|GetLength) 1))
        (Variables|Default|Sety _index_3)
        (CallFunction|PlaceBlockOfType (Math|Vector|MakeVector (* (Variables|Default|GetX) 1e+02) (* (Variables|Default|Gety) 1e+02) (* (Variables|Default|GetZ) 1e+02)) "NewEnumerator9")))))

(fn ConstructionScript
  (|CallParentFunction))

(fn RunCode
  (CallFunction|PuzzleSolution))