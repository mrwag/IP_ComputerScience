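; BP_NL_06_Start is a nested-loops lesson puzzle that builds a stepped pyramid of blocks when RunCode calls PuzzleSolution.
; PuzzleSolution runs three nested loops over layer, X and Y, placing one block type on a 100-unit grid through PlaceBlockOfType.
; The layer index insets both horizontal ranges from the FloorX and FloorY bounds, so each higher layer shrinks by one block per side.
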(event Custom|PuzzleSolution
  (for _index (range 0 5)
    (Variables|Default|SetZ _index)
    (for _index_2 (range (Variables|Default|GetZ) (- (- (Variables|Default|GetFloorX) 1) (Variables|Default|GetZ)))
      (Variables|Default|SetX _index_2)
      (for _index_3 (range (Variables|Default|GetZ) (- (- (Variables|Default|GetFloorY) 1) (Variables|Default|GetZ)))
        (Variables|Default|Sety _index_3)
        (CallFunction|PlaceBlockOfType (Math|Vector|MakeVector (* (Variables|Default|GetX) 1e+02) (* (Variables|Default|Gety) 1e+02) (* (Variables|Default|GetZ) 1e+02)) "NewEnumerator3")))))

(fn ConstructionScript
  (|CallParentFunction))

(fn RunCode
  (CallFunction|PuzzleSolution))